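; BasicEnemy is a patrolling enemy that shuttles between two reference actors, Point1 and Point2, and hurts the player on contact.
; Each Tick it sweeps its Cube toward the current target by Speed, not scaled by delta time, and switches targets when within range.
; A Cube hit against a SideScrollerCharacter applies a fixed amount of damage.
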(event OnComponentHit(Cube)
  (params (HitComponent :type Primitive%20Component%20Object%20Reference) (OtherActor :type Actor%20Object%20Reference) (OtherComp :type Primitive%20Component%20Object%20Reference) (NormalImpulse :type Vector :default "0, 0, 0") (Hit :type Hit%20Result%20Structure%20%28by%20ref%29))
  (bind _asside_scroller_character (Utilities|Casting|CastToSideScrollerCharacter OtherActor))
  (Game|Damage|ApplyDamage _asside_scroller_character 1e+01 0 self))

(event EventBeginPlay
  (Variables|Default|SetPoint (Variables|Default|GetPoint1)))

(event Collision|EventActorBeginOverlap
  (params (OtherActor :type Actor%20Object%20Reference)))

(event EventTick
  (params (DeltaSeconds :type Float%20%28single-precision%29))
  (bind _cube (Variables|Default|GetCube))
  (bind _returnvalue (Transformation|GetWorldLocation _cube))
  (Transformation|AddWorldOffset (Variables|Default|GetCube) (* (Math|Vector|GetUnitDirection(Vector) _returnvalue (Transformation|GetActorLocation (Variables|Default|GetPoint))) (Variables|Default|GetSpeed)) true false)
  (Utilities|FlowControl|Sequence
    (:then_0
      (if (<= (Math|Vector|VectorLength (- (Transformation|GetActorLocation (Variables|Default|GetPoint1)) _returnvalue)) 1e+02)
        (Variables|Default|SetPoint (Variables|Default|GetPoint2))))
    (:then_1
      (if (<= (Math|Vector|VectorLength (- (Transformation|GetActorLocation (Variables|Default|GetPoint2)) _returnvalue)) 1e+02)
        (Variables|Default|SetPoint (Variables|Default|GetPoint1))))))

(fn ConstructionScript)